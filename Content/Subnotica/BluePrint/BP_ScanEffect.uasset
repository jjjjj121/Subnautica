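; BP_ScanEffect is an actor that animates a pulsing scan effect by repeatedly stretching and shrinking along its Z axis.
; On BeginPlay it starts a looping timer for Add Scale, which grows the root's Z scale by world delta seconds.
; Add Scale and Minus Scale hand off to each other by swapping timers at upper and lower limits, creating an endless ping-pong.
; The mesh's overlap event does nothing.
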(event OnComponentBeginOverlap(StaticMesh)
  (params (OverlappedComponent :type Primitive%20Component%20Object%20Reference) (OtherActor :type Actor%20Object%20Reference) (OtherComp :type Primitive%20Component%20Object%20Reference) (OtherBodyIndex :type Integer) (bFromSweep :type Boolean) (SweepResult :type Hit%20Result%20Structure%20%28by%20ref%29)))

(event EventBeginPlay
  (Utilities|Time|SetTimerbyFunctionName 0 "Add Scale" 0.01 true))

(event EventTick
  (params (DeltaSeconds :type Float%20%28single-precision%29)))

(fn ConstructionScript)

(fn AddScale
  (if (>= (Variables|Default|GetScale%20Value) 1.0)
    (Utilities|Time|ClearTimerbyFunctionName 0 "Add Scale")
    (Utilities|Time|SetTimerbyFunctionName 0 "Minus Scale" 0.01 true)
    (else
      (bind _output_get (Variables|Default|SetScale%20Value (+ (Variables|Default|GetScale%20Value) (Utilities|Time|GetWorldDeltaSeconds))))
      (Transformation|SetRelativeScale3D (Variables|Default|GetDefaultSceneRoot) (Math|Vector|MakeVector 1.0 1.0 _output_get)))))

(fn MinusScale
  (if (<= (Variables|Default|GetScale%20Value) 0.1)
    (Utilities|Time|ClearTimerbyFunctionName 0 "Minus Scale")
    (Utilities|Time|SetTimerbyFunctionName 0 "Add Scale" 0.01 true)
    (else
      (bind _output_get (Variables|Default|SetScale%20Value (- (Variables|Default|GetScale%20Value) (Utilities|Time|GetWorldDeltaSeconds))))
      (Transformation|SetRelativeScale3D (Variables|Default|GetDefaultSceneRoot) (Math|Vector|MakeVector 1.0 1.0 _output_get)))))