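; Building_Room02 is a building room Blueprint that tracks whether the VR player is inside the house.
; When an SN_VRPawn stops overlapping Door1 or Door2, it reads the pawn's CharacterState and sets IsInHouse on the Ocean reference.
; One specific state clears the flag and any other state sets it, with identical logic duplicated for both doors.
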(event OnComponentEndOverlap(Door2)
  (params (OverlappedComponent :type Primitive%20Component%20Object%20Reference) (OtherActor :type Actor%20Object%20Reference) (OtherComp :type Primitive%20Component%20Object%20Reference) (OtherBodyIndex :type Integer))
  (bind _assn_vrpawn (Utilities|Casting|CastToSN_VRPawn OtherActor))
  (if (Utilities|Enum|Equal(Enum) (Variables|/Game/Subnotica/GameMode/SN_VRPawn.SN_VRPawn_C|GetCharacter%20State _assn_vrpawn) "NewEnumerator1")
    (Variables|/Game/CartoonWaterShader/Blueprints/CartoonWaterBlueprints/BP_CartoonWater_Ocean.BP_CartoonWater_Ocean_C|SetIs%20In%20House (Variables|Default|GetOcean) false)
    (else
      (Variables|/Game/CartoonWaterShader/Blueprints/CartoonWaterBlueprints/BP_CartoonWater_Ocean.BP_CartoonWater_Ocean_C|SetIs%20In%20House (Variables|Default|GetOcean) true))))

(event OnComponentEndOverlap(Door1)
  (params (OverlappedComponent :type Primitive%20Component%20Object%20Reference) (OtherActor :type Actor%20Object%20Reference) (OtherComp :type Primitive%20Component%20Object%20Reference) (OtherBodyIndex :type Integer))
  (bind _assn_vrpawn (Utilities|Casting|CastToSN_VRPawn OtherActor))
  (if (Utilities|Enum|Equal(Enum) (Variables|/Game/Subnotica/GameMode/SN_VRPawn.SN_VRPawn_C|GetCharacter%20State _assn_vrpawn) "NewEnumerator1")
    (Variables|/Game/CartoonWaterShader/Blueprints/CartoonWaterBlueprints/BP_CartoonWater_Ocean.BP_CartoonWater_Ocean_C|SetIs%20In%20House (Variables|Default|GetOcean) false)
    (else
      (Variables|/Game/CartoonWaterShader/Blueprints/CartoonWaterBlueprints/BP_CartoonWater_Ocean.BP_CartoonWater_Ocean_C|SetIs%20In%20House (Variables|Default|GetOcean) true))))

(event EventBeginPlay
  (|CallParentFunction) ; 지금 이 노드는 비활성 상태입니다. \n핀을 끌어서 다른 노드를 연결하면 활성화됩니다.
)

(event Collision|EventActorBeginOverlap
  (params (OtherActor :type Actor%20Object%20Reference))
  (|CallParentFunction OtherActor) ; 지금 이 노드는 비활성 상태입니다. \n핀을 끌어서 다른 노드를 연결하면 활성화됩니다.
)

(event EventTick
  (params (DeltaSeconds :type Float%20%28single-precision%29))
  (|CallParentFunction DeltaSeconds) ; 지금 이 노드는 비활성 상태입니다. \n핀을 끌어서 다른 노드를 연결하면 활성화됩니다.
)

(fn ConstructionScript
  (|CallParentFunction))