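; Building actor for the Subnotica game, providing door open/close behavior and access to its collision boxes.
; On BeginPlay it caches the BP_CartoonWater_Ocean actor.
; Open Door clears the door's second material slot, disables collision and sets a timer by name for Close Door, which takes a Door parameter and restores both.
; Get Collision Array returns all box components, with Result always false.
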(event EventBeginPlay
  (bind _returnvalue (Actor|GetActorOfClass "/Game/CartoonWaterShader/Blueprints/CartoonWaterBlueprints/BP_CartoonWater_Ocean.BP_CartoonWater_Ocean_C"))
  (Utilities|IsValid _returnvalue
    (:Is%20Valid
      (Variables|Default|SetOcean _returnvalue))))

(event Collision|EventActorBeginOverlap
  (params (OtherActor :type Actor%20Object%20Reference)))

(event EventTick
  (params (DeltaSeconds :type Float%20%28single-precision%29)))

(fn ConstructionScript)

(fn OpenDoor
  (params (Door :type Primitive%20Component%20Object%20Reference))
  (Rendering|Material|SetMaterial Door 1 0)
  (Collision|SetCollisionEnabled Door "NoCollision")
  (Utilities|Time|SetTimerbyFunctionName 0 "Close Door" 5.0))

(fn CloseDoor
  (params (Door :type Primitive%20Component%20Object%20Reference))
  (Rendering|Material|SetMaterial Door 1 "/Game/Subnotica/Effect/Basic_Color_Inst.Basic_Color_Inst")
  (Collision|SetCollisionEnabled Door "QueryAndPhysics"))

(fn GetCollisionArray
  (return (Actor|GetComponentsByClass "/Script/Engine.BoxComponent") false))