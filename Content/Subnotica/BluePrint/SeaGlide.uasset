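; VR Seaglide item that propels the player pawn while both handles are held.
; The first controller within a handle's sphere snaps it to that hand; a second grab enables trigger input, which offsets the pawn along the glider's axis.
; Tick steers the glider using look-at rotation between the controllers and the second hand's pitch.
; Releasing over the watch's inventory stores the item and destroys the actor; otherwise, releasing the first hand drops it with physics.
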(event EventBeginPlay
  (bind _returnvalue (Utilities|GetDataTableRow "/Game/Subnotica/Data/DT_Item.DT_Item" "SeaGlider")
    (:then
      (Variables|Default|SetST_Item _returnvalue)
      (bind _assn_vrpawn (Utilities|Casting|CastToSN_VRPawn (Game|Player|GetPlayerPawn 0)))
      (Variables|Default|SetOwn%20Pawn _assn_vrpawn)
      (bind _watch (Variables|Default|GetWatch)
        (:then
          (Variables|/Game/Subnotica/BluePrint/Watch/Watch.Watch_C|SetSeaGlide _watch self))
        (:else)))))

(event EventTick
  (params (DeltaSeconds :type Float%20%28single-precision%29))
  (bind _first_motion_controller (Variables|Default|GetFirst%20Motion%20Controller))
  (bind _second_motion_controller (Variables|Default|GetSecond%20Motion%20Controller))
  (bind _first_motion_controller_2 (Variables|Default|GetFirst%20Motion%20Controller))
  (bind _second_motion_controller_2 (Variables|Default|GetSecond%20Motion%20Controller))
  (bind _returnvalue (Transformation|GetWorldLocation _second_motion_controller))
  (bind _returnvalue_2 (Transformation|GetWorldLocation _first_motion_controller_2))
  (bind _returnvalue_3 (Transformation|GetWorldLocation _second_motion_controller_2))
  (bind _returnvalue_4 (Transformation|GetWorldLocation _first_motion_controller))
  (bind _returnvalue_5 (Math|Rotator|FindLookatRotation _returnvalue_2 _returnvalue))
  (bind _returnvalue_6 (Math|Rotator|FindLookatRotation _returnvalue_4 _returnvalue_3))
  (bind _returnvalue_7 (Math|Rotator|CombineRotators _returnvalue_5 "0,90.000000, 0"))
  (bind _returnvalue_8 (Math|Rotator|CombineRotators _returnvalue_6 "0,-90.000000, 0"))
  ;[1 1 1] Tick - Rotate First Handle
  (if (and (Utilities|IsValid (Variables|Default|GetFirst%20Motion%20Controller)) (Utilities|IsValid (Variables|Default|GetSecond%20Motion%20Controller)))
    (if (Utilities|String|Contains (Utilities|GetDisplayName (Variables|Default|GetFirst%20Motion%20Controller)) "Right") ; 오른손? 왼손?
      (Transformation|SetActorRotation (Math|Rotator|MakeRotator (.roll _returnvalue_8) (* (.pitch (Transformation|GetWorldRotation _second_motion_controller_2)) -1.0) (.yaw _returnvalue_8)))
      (else
        (Transformation|SetActorRotation (Math|Rotator|MakeRotator (.roll _returnvalue_7) (* (.pitch (Transformation|GetWorldRotation _second_motion_controller)) -1.0) (.yaw _returnvalue_7)))))))

(event EventGrab
  (params (Motion%20Controller :type Motion%20Controller%20Component%20Object%20Reference))
  (bind _glidercollision_left (Variables|Default|GetGliderCollision_Left))
  (bind _glidercollision_right (Variables|Default|GetGliderCollision_Right))
  (bind _glidercollision_left_2 (Variables|Default|GetGliderCollision_Left))
  (bind _glidercollision_right_2 (Variables|Default|GetGliderCollision_Right))
  (bind _glidercollision_right_3 (Variables|Default|GetGliderCollision_Right))
  (bind _glidercollision_left_3 (Variables|Default|GetGliderCollision_Left))
  ;[1 1 1] Grab Event
  (Utilities|IsValid (Variables|Default|GetFirst%20Motion%20Controller) ; 이미 잡고 있는 손이 있는가?
    (:Is%20Valid
      (Variables|Default|SetIs%20Grab%20All%20Handle? true)
      (CallFunction|PlayerInputEnable)
      (if (Utilities|String|Contains (Utilities|GetDisplayName Motion%20Controller) "Right") ; 왼손? 오른손?
        (if (<= (Math|Vector|Distance(Vector) (Transformation|GetWorldLocation Motion%20Controller) (Transformation|GetWorldLocation _glidercollision_right_3)) (Variables|/Script/Engine.SphereComponent|GetSphereRadius _glidercollision_right_3))
          (Variables|Default|SetSecond%20Motion%20Controller Motion%20Controller))
        (elif (<= (Math|Vector|Distance(Vector) (Transformation|GetWorldLocation Motion%20Controller) (Transformation|GetWorldLocation _glidercollision_left_3)) (Variables|/Script/Engine.SphereComponent|GetSphereRadius _glidercollision_left_3))
          (Variables|Default|SetSecond%20Motion%20Controller Motion%20Controller))))
    (:Is%20Not%20Valid
      (if (Utilities|String|Contains (Utilities|GetDisplayName Motion%20Controller) "Right") ; 왼손? 오른손?
        (if (<= (Math|Vector|Distance(Vector) (Transformation|GetWorldLocation Motion%20Controller) (Transformation|GetWorldLocation _glidercollision_right)) (Variables|/Script/Engine.SphereComponent|GetSphereRadius _glidercollision_right))
          (bind _output_get (Variables|Default|SetFirst%20Motion%20Controller Motion%20Controller))
          (Transformation|AttachComponentToComponent (Transformation|GetAttachParent (Variables|Default|GetGliderCollision_Right)) _output_get "None" "SnapToTarget" "SnapToTarget" "KeepWorld" true) ; Snap
          (Transformation|SetRelativeRotation (Transformation|GetAttachParent _glidercollision_right_2) (Class|KismetMathLibrary|NegateRotator (Variables|/Script/Engine.SceneComponent|GetRelativeRotation _glidercollision_right_2)) false true)
          (Transformation|SetWorldLocation (Transformation|GetAttachParent (Variables|Default|GetGliderCollision_Right)) (+ (Transformation|GetWorldLocation _output_get) (* (- (Transformation|GetWorldLocation (Variables|Default|GetGliderCollision_Right)) (Transformation|GetWorldLocation (Transformation|GetAttachParent (Variables|Default|GetGliderCollision_Right)))) -1.0)) false true))
        (elif (<= (Math|Vector|Distance(Vector) (Transformation|GetWorldLocation Motion%20Controller) (Transformation|GetWorldLocation _glidercollision_left)) (Variables|/Script/Engine.SphereComponent|GetSphereRadius _glidercollision_left))
          (bind _output_get_2 (Variables|Default|SetFirst%20Motion%20Controller Motion%20Controller))
          (Transformation|AttachComponentToComponent (Transformation|GetAttachParent (Variables|Default|GetGliderCollision_Left)) _output_get_2 "None" "SnapToTarget" "SnapToTarget" "KeepWorld" true) ; Snap
          (Transformation|SetRelativeRotation (Transformation|GetAttachParent _glidercollision_left_2) (Class|KismetMathLibrary|NegateRotator (Variables|/Script/Engine.SceneComponent|GetRelativeRotation _glidercollision_left_2)) false true)
          (Transformation|SetWorldLocation (Transformation|GetAttachParent (Variables|Default|GetGliderCollision_Left)) (+ (Transformation|GetWorldLocation _output_get_2) (* (- (Transformation|GetWorldLocation (Variables|Default|GetGliderCollision_Left)) (Transformation|GetWorldLocation (Transformation|GetAttachParent (Variables|Default|GetGliderCollision_Left)))) -1.0)) false true))))))

(event EventRelease
  (params (Motion%20Controller :type Motion%20Controller%20Component%20Object%20Reference))
  (bind _glidercollision_right (Variables|Default|GetGliderCollision_Right))
  (bind _glidercollision_right_2 (Variables|Default|GetGliderCollision_Right))
  (bind _glidercollision_left (Variables|Default|GetGliderCollision_Left))
  (bind _glidercollision_left_2 (Variables|Default|GetGliderCollision_Left))
  (bind _inventory_widget (Variables|Default|GetInventory%20Widget))
  ;[1 1 1] Drop Event
  (Utilities|FlowControl|Sequence
    (:then_0
      (bind _watch (Variables|Default|GetWatch)
        (:then
          (if (Variables|/Game/Subnotica/BluePrint/Watch/Watch.Watch_C|GetQ_InventoryOverlap _watch)
            ;;[0 0.5616 1] 인벤토리에 추가
            (Utilities|IsValid _inventory_widget
              (:Is%20Valid
                (Default|UpdateItem _inventory_widget (Variables|Default|GetST_Item))
                (Variables|/Game/Subnotica/BluePrint/Watch/Watch.Watch_C|SetIs%20Get%20SeaGlide _watch true)
                (Actor|DestroyActor)))))
        (:else)))
    (:then_1
      (if (== Motion%20Controller (Variables|Default|GetFirst%20Motion%20Controller)) ; 첫번째로 집은 손임?
        (Variables|Default|SetFirst%20Motion%20Controller 0) ; 둘 다 떨어지게
        (Variables|Default|SetSecond%20Motion%20Controller 0)
        (Transformation|DetachFromActor "KeepWorld" "KeepWorld" "KeepWorld")
        (Variables|Default|SetIs%20Grab%20All%20Handle? false)
        (bind _seaglide (Variables|Default|GetSeaGlide)
          (:then
            (Physics|SetSimulatePhysics _seaglide true)
            (CallFunction|PlayerIntputDisable)
            (bind _watch_2 (Variables|Default|GetWatch)
              (:then
                (Variables|/Game/Subnotica/BluePrint/Watch/Watch.Watch_C|SetSeaGlide _watch_2 self))
              (:else)))
          (:else))))
    (:then_2
      (if (== Motion%20Controller (Variables|Default|GetSecond%20Motion%20Controller)) ; 나중에 집은 손임?
        (Variables|Default|SetSecond%20Motion%20Controller 0)
        (bind _first_motion_controller (Variables|Default|GetFirst%20Motion%20Controller)
          (:then
            (if (Utilities|String|Contains (Utilities|GetDisplayName _first_motion_controller) "Right") ; 오른손? 왼손?
              (Transformation|SetRelativeRotation (Transformation|GetAttachParent _glidercollision_right) (Class|KismetMathLibrary|NegateRotator (Variables|/Script/Engine.SceneComponent|GetRelativeRotation _glidercollision_right)) false true)
              (Transformation|SetWorldLocation (Transformation|GetAttachParent (Variables|Default|GetGliderCollision_Right)) (+ (Transformation|GetWorldLocation _first_motion_controller) (* (- (Transformation|GetWorldLocation _glidercollision_right_2) (Transformation|GetWorldLocation (Transformation|GetAttachParent _glidercollision_right_2))) -1.0)) false true)
              (else
                (Transformation|SetRelativeRotation (Transformation|GetAttachParent _glidercollision_left) (Class|KismetMathLibrary|NegateRotator (Variables|/Script/Engine.SceneComponent|GetRelativeRotation _glidercollision_left)) false true)
                (Transformation|SetWorldLocation (Transformation|GetAttachParent (Variables|Default|GetGliderCollision_Left)) (+ (Transformation|GetWorldLocation _first_motion_controller) (* (- (Transformation|GetWorldLocation _glidercollision_left_2) (Transformation|GetWorldLocation (Transformation|GetAttachParent _glidercollision_left_2))) -1.0)) false true)))
            (Variables|Default|SetIs%20Grab%20All%20Handle? false)
            (CallFunction|PlayerIntputDisable))
          (:else
            (Transformation|DetachFromActor "KeepWorld" "KeepWorld" "KeepWorld")
            (Variables|Default|SetIs%20Grab%20All%20Handle? false)
            (Physics|SetSimulatePhysics (Variables|Default|GetSeaGlide) true)
            (CallFunction|PlayerIntputDisable)
            (bind _watch_3 (Variables|Default|GetWatch)
              (:then
                (Variables|/Game/Subnotica/BluePrint/Watch/Watch.Watch_C|SetSeaGlide _watch_3 0))
              (:else))))))))

(event Input|AxisEvents|InputAxisTriggerAxisLeft
  (params (AxisValue :type Float%20%28single-precision%29))
  ;[1 1 1] SeaGlide Move Forward
  (if (Variables|Default|GetIs%20Grab%20All%20Handle?) ; 양손 다 잡고 있는가?
    (Transformation|AddActorWorldOffset (Variables|Default|GetOwn%20Pawn) (* (* (Transformation|GetActorForwardVector) AxisValue) -1e+01))))

(event Input|AxisEvents|InputAxisTriggerAxisRight
  (params (AxisValue :type Float%20%28single-precision%29))
  ;[1 1 1] SeaGlide Move Forward
  (if (Variables|Default|GetIs%20Grab%20All%20Handle?) ; 양손 다 잡고 있는가?
    (Transformation|AddActorWorldOffset (Variables|Default|GetOwn%20Pawn) (* (* (Transformation|GetActorForwardVector) AxisValue) -1e+01))))

(fn ConstructionScript)

(fn PlayerInputEnable
  (Input|EnableInput (Game|GetPlayerController 0)))

(fn PlayerIntputDisable
  (Input|DisableInput (Game|GetPlayerController 0)))

(fn DragEvent
  (return false))

(fn DropItem
  (Variables|Default|SetInventory%20Widget 0)
  (Variables|Default|SetWatch 0)
  (return false))

(fn GetItem
  (params (Own%20Pawn :type SN%20VR%20Pawn%20Object%20Reference) (Inventory%20Widget :type Inventory%20Widget%20Object%20Reference) (Watch :type Watch%20Object%20Reference))
  (Variables|Default|SetInventory%20Widget Inventory%20Widget)
  (Variables|Default|SetWatch Watch)
  (Variables|/Game/Subnotica/BluePrint/Watch/Watch.Watch_C|SetSeaGlide Watch self)
  (return false))

(fn PressTrigger
  (return false))

(fn RealeseTrigger
  (return false))