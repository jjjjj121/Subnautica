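; Grabbable VR scanner for placing underwater buildings, which returns to the inventory when dropped over the watch.
; In building mode a line trace positions a preview of the selected DT_Build piece, snapping to BuildCollision sockets.
; Overlap and ocean-height checks swap the preview material and gate the trigger, which asks the pawn to check build items.
; SpawnBuild spawns the piece, then disables nearby BuildCollision and hides Door components.
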(event OnGrabbed(GrabComponent)
  (params (Motion%20Controller :type Motion%20Controller%20Component%20Object%20Reference))
  ;[0.07292 0.07292 0.07292] Set Input & Building Mode
  (Input|EnableInput (Game|GetPlayerController 0))
  (bind _watch (Variables|Default|GetWatch)
    (:then
      (Variables|/Game/Subnotica/BluePrint/Watch/Watch.Watch_C|SetScanner _watch self))
    (:else)))

(event OnDropped(GrabComponent)
  (bind _inventory_widget (Variables|Default|GetInventory%20Widget))
  ;[0.07292 0.07292 0.07292] Set Input & Building Mode
  (Input|DisableInput (Game|GetPlayerController 0))
  (Variables|Default|SetIs%20Building%20Mode false)
  (bind _watch (Variables|Default|GetWatch)
    (:then
      (Variables|/Game/Subnotica/BluePrint/Watch/Watch.Watch_C|SetScanner _watch 0)
      (if (Variables|/Game/Subnotica/BluePrint/Watch/Watch.Watch_C|GetQ_InventoryOverlap _watch)
        ;;[0 0.5616 1] 인벤토리에 추가
        (Utilities|IsValid _inventory_widget
          (:Is%20Valid
            (Default|UpdateItem _inventory_widget (Variables|Default|GetST_Item))
            (Variables|/Game/Subnotica/BluePrint/Watch/Watch.Watch_C|SetIs%20Get%20Scanner _watch true)
            (Actor|DestroyActor)))))
    (:else)))

(event Custom|Reset%20Once%20Mode%20On
  (Utilities|FlowControl|DoOnce false) ; enters at Reset
)

(event Custom|Reset%20Once%20Mode%20Off
  (Utilities|FlowControl|DoOnce false) ; enters at Reset
)

(event Custom|Change%20Impossible%20Preview
  ;[0.1406 0.1406 0.1406] Change Preview
  (Utilities|FlowControl|DoOnce false
    (:Completed
      (CallFunction|SetBuildingPreview (Variables|/Script/Engine.StaticMeshComponent|GetStaticMesh (Variables|Default|GetBuliding%20Preview)) "/Game/Subnotica/Effect/Build/Master_Glass_Mat_Inst.Master_Glass_Mat_Inst")
      (CallFunction|ResetPossible)
      (Variables|Default|SetIs%20Possible%20Build false))))

(event Custom|Reset%20Impossible
  ;[0.1406 0.1406 0.1406] Change Preview
  (Utilities|FlowControl|DoOnce false) ; enters at Reset
)

(event Custom|Change%20Possible%20Preview
  ;[0.1406 0.1406 0.1406] Change Preview
  (Utilities|FlowControl|DoOnce false
    (:Completed
      (CallFunction|SetBuildingPreview (Variables|/Script/Engine.StaticMeshComponent|GetStaticMesh (Variables|Default|GetBuliding%20Preview)) "/Game/Subnotica/Effect/Build/WM_GlassClean_a.WM_GlassClean_a")
      (CallFunction|ResetImpossible)
      (Variables|Default|SetIs%20Possible%20Build true))))

(event Custom|Reset%20Possible
  ;[0.1406 0.1406 0.1406] Change Preview
  (Utilities|FlowControl|DoOnce false) ; enters at Reset
)

(event Custom|Spawn%20Build
  (bind _impact_point (Variables|Default|GetImpact%20Point))
  (Game|SpawnActorfromClass (.BuildActor (Utilities|Struct|BreakST_Build (Variables|Default|GetST%20Build))) (Transformation|GetWorldTransform (Variables|Default|GetBuliding%20Preview)) "Undefined" 0 0)
  (bind _outhits (Collision|MultiSphereTraceForObjects _impact_point _impact_point 1e+02 (Utilities|Array|MakeArray "ObjectTypeQuery2" "ObjectTypeQuery1") false 0 "ForDuration"))
  (bind _array_element (Utilities|Array|ForEachLoopwithBreak _outhits)
    (:LoopBody
      (Utilities|FlowControl|Sequence
        (:then_0
          (if (Utilities|String|Contains (Utilities|GetDisplayName (.HitComponent (Collision|BreakHitResult _array_element))) "BuildCollision")
            (Collision|SetCollisionEnabled (.HitComponent (Collision|BreakHitResult _array_element)) "NoCollision")))
        (:then_1
          (if (Utilities|String|Contains (Utilities|GetDisplayName (.HitComponent (Collision|BreakHitResult _array_element))) "Door")
            (Development|PrintString (Utilities|GetDisplayName (.HitComponent (Collision|BreakHitResult _array_element))) true true "(R=1.000000,G=0.000000,B=0.198145,A=1.000000)" 1e+01)
            (Rendering|SetVisibility (.HitComponent (Collision|BreakHitResult _array_element)) false false)
            (Collision|SetCollisionEnabled (.HitComponent (Collision|BreakHitResult _array_element)) "NoCollision")))))))

(event EventBeginPlay
  (CallFunction|InitPawn)
  (CallFunction|InitBuildArray)
  (CallFunction|InitVariable)
  (bind _asbuild_info (Utilities|Casting|CastToBuild_Info (UserInterface|GetWidget (Variables|Default|GetWidget_Info))))
  (Variables|Default|SetBuild%20Widget _asbuild_info)
  (bind _returnvalue (Actor|GetActorOfClass "/Game/CartoonWaterShader/Blueprints/CartoonWaterBlueprints/BP_CartoonWater_Ocean.BP_CartoonWater_Ocean_C"))
  (Utilities|IsValid _returnvalue
    (:Is%20Valid
      (Variables|Default|SetOcean _returnvalue))))

(event EventTick
  (params (DeltaSeconds :type Float%20%28single-precision%29))
  (if (Variables|Default|GetIs%20Building%20Mode) ; 빌딩 모드인가?
    (Utilities|FlowControl|Sequence
      (:then_0
        (Utilities|FlowControl|DoOnce false ; Preview On
          (:Completed
            (Rendering|SetVisibility (Variables|Default|GetBuliding%20Preview) true false)
            (Collision|SetCollisionEnabled (Variables|Default|GetCollision%20Box) "QueryAndPhysics")
            (CallFunction|ResetOnceModeon))))
      (:then_1
        (bind _on_build_collision_ (CallFunction|SetLocationBuildingPreview))
        (bind _is_possible_build (CallFunction|CheckPossibleBuild _on_build_collision_))
        (bind _under_water_ (CallFunction|CheckUnderWater))
        (if (and _under_water_ _is_possible_build) ; 건축 가능한 위치인가?
          (CallFunction|ChangePossiblePreview)
          (else
            (CallFunction|ChangeImpossiblePreview)))))
    (else
      (Utilities|FlowControl|DoOnce false ; Preview Off
        (:Completed
          (Rendering|SetVisibility (Variables|Default|GetBuliding%20Preview) false false)
          (Collision|SetCollisionEnabled (Variables|Default|GetCollision%20Box) "NoCollision")
          (CallFunction|ResetOnceModeOff))))))

(event Input|ActionEvents|InputActionBuildingMode
  (params (Key :type Key%20Structure :default "None"))
  ;[0.07292 0.07292 0.07292] Set Input & Building Mode
  (:Pressed
    (if (Variables|Default|GetIs%20Building%20Mode)
      (Variables|Default|SetIs%20Building%20Mode false)
      (else
        (Variables|Default|SetIs%20Building%20Mode true)))))

(event Input|ActionEvents|InputActionTriggerRight
  (params (Key :type Key%20Structure :default "None"))
  (:Pressed
    (if (Variables|Default|GetIs%20Building%20Mode)
      (if (Variables|Default|GetIs%20Possible%20Build)
        (bind _own_vrpawn (Variables|Default|GetOwn%20VRPawn)
          (:then
            (Default|CheckBuildItem _own_vrpawn (Variables|Default|GetST%20Build) self))
          (:else))))))

(event Input|AxisEvents|InputAxisMovementAxisRight_Y
  (params (AxisValue :type Float%20%28single-precision%29))
  ;[0.09896 0.09896 0.09896] Change Preview Mesh
  ;;[0.08854 0.08854 0.08854] VR
  (if (CallFunction|IsAxisGreaterThanDeadzone AxisValue)
    (Utilities|FlowControl|DoOnce false :!label _label
      (:Completed
        (if (> AxisValue 0.0)
          (if (Variables|Default|GetIs%20Building%20Mode) ; Build Mode 인지?
            (if (> (+ (Variables|Default|GetArray%20Index) 1) (Utilities|GetArrayMaxIndex)) ; Max Index 보다 커졌다면 Min로
              (Variables|Default|SetArray%20Index 0)
              (else
                (Variables|Default|SetArray%20Index (+ (Variables|Default|GetArray%20Index) 1))))
            (bind _output_get (Variables|Default|SetST%20Build (Utilities|Array|Get(acopy) (Variables|Default|GetST_BuildArray) (Variables|Default|GetArray%20Index)) :!label _label_2))
            (Components|StaticMesh|SetStaticMesh (Variables|Default|GetBuliding%20Preview) (.StaticMesh (Utilities|Struct|BreakST_Build _output_get)))
            (Default|UpdateInfo (Variables|Default|GetBuild%20Widget) (Variables|Default|GetST%20Build)))
          (elif (Variables|Default|GetIs%20Building%20Mode) ; Build Mode 인지?
            (if (< (- (Variables|Default|GetArray%20Index) 1) 0) ; Min Index 보다 작아졌다면 Max로
              (Variables|Default|SetArray%20Index (Utilities|GetArrayMaxIndex))
              (goto _label_2)
              (else
                (Variables|Default|SetArray%20Index (- (Variables|Default|GetArray%20Index) 1))
                (goto _label_2)))))))
    (else
      (goto _label Reset))))

(event Input|AxisEvents|InputAxisMovementAxisRight_X
  (params (AxisValue :type Float%20%28single-precision%29))
  (bind _buliding_preview (Variables|Default|GetBuliding%20Preview))
  (bind _buliding_preview_2 (Variables|Default|GetBuliding%20Preview))
  (bind _returnvalue (Transformation|GetWorldRotation _buliding_preview))
  (bind _returnvalue_2 (Transformation|GetWorldRotation _buliding_preview_2))
  ;[0.1042 0.1042 0.1042] Change Previw Rotation
  ;;[0.08854 0.08854 0.08854] VR
  (if (CallFunction|IsAxisGreaterThanDeadzone AxisValue)
    (Utilities|FlowControl|DoOnce false :!label _label
      (:Completed
        (if (> AxisValue 0.0)
          (if (Variables|Default|GetIs%20Building%20Mode) ; Build Mode 인지?
            (Transformation|SetWorldRotation _buliding_preview_2 (Math|Rotator|MakeRotator (.roll _returnvalue_2) (.pitch _returnvalue_2) (+ (.yaw _returnvalue_2) 9e+01)) false false))
          (elif (Variables|Default|GetIs%20Building%20Mode) ; Build Mode 인지?
            (Transformation|SetWorldRotation _buliding_preview (Math|Rotator|MakeRotator (.roll _returnvalue) (.pitch _returnvalue) (- (.yaw _returnvalue) 9e+01)) false false)))))
    (else
      (goto _label Reset))))

(event Input|MouseEvents|LeftMouseButton
  (params (Key :type Key%20Structure :default "None")))

(event Input|MouseEvents|MouseWheelUp
  (params (Key :type Key%20Structure :default "None")))

(event Input|MouseEvents|MouseWheelDown
  (params (Key :type Key%20Structure :default "None")))

(event Input|KeyboardEvents|E
  (params (Key :type Key%20Structure :default "None"))
  (bind _buliding_preview (Variables|Default|GetBuliding%20Preview))
  (bind _returnvalue (Transformation|GetWorldRotation _buliding_preview))
  ;[0.1042 0.1042 0.1042] Change Previw Rotation
  (:Pressed
    (if (Variables|Default|GetIs%20Building%20Mode) ; Build Mode 인지?
      (Transformation|SetWorldRotation _buliding_preview (Math|Rotator|MakeRotator (.roll _returnvalue) (.pitch _returnvalue) (+ (.yaw _returnvalue) 9e+01)) false false))))

(event Input|KeyboardEvents|Q
  (params (Key :type Key%20Structure :default "None"))
  (bind _buliding_preview (Variables|Default|GetBuliding%20Preview))
  (bind _returnvalue (Transformation|GetWorldRotation _buliding_preview))
  ;[0.1042 0.1042 0.1042] Change Previw Rotation
  (:Pressed
    (if (Variables|Default|GetIs%20Building%20Mode) ; Build Mode 인지?
      (Transformation|SetWorldRotation _buliding_preview (Math|Rotator|MakeRotator (.roll _returnvalue) (.pitch _returnvalue) (- (.yaw _returnvalue) 9e+01)) false false))))

(event Input|MouseEvents|RightMouseButton
  (params (Key :type Key%20Structure :default "None")))

(event Input|KeyboardEvents|R
  (params (Key :type Key%20Structure :default "None"))
  ;[0.09896 0.09896 0.09896] Change Preview Mesh
  (:Pressed
    (if (Variables|Default|GetIs%20Building%20Mode) ; Build Mode 인지?
      (if (< (- (Variables|Default|GetArray%20Index) 1) 0) ; Min Index 보다 작아졌다면 Max로
        (Variables|Default|SetArray%20Index (Utilities|GetArrayMaxIndex))
        (else
          (Variables|Default|SetArray%20Index (- (Variables|Default|GetArray%20Index) 1))))
      (bind _output_get (Variables|Default|SetST%20Build (Utilities|Array|Get(acopy) (Variables|Default|GetST_BuildArray) (Variables|Default|GetArray%20Index))))
      (Components|StaticMesh|SetStaticMesh (Variables|Default|GetBuliding%20Preview) (.StaticMesh (Utilities|Struct|BreakST_Build _output_get)))
      (Default|UpdateInfo (Variables|Default|GetBuild%20Widget) (Variables|Default|GetST%20Build)))))

(event Input|KeyboardEvents|T
  (params (Key :type Key%20Structure :default "None"))
  ;[0.09896 0.09896 0.09896] Change Preview Mesh
  (:Pressed
    (if (Variables|Default|GetIs%20Building%20Mode) ; Build Mode 인지?
      (if (> (+ (Variables|Default|GetArray%20Index) 1) (Utilities|GetArrayMaxIndex)) ; Max Index 보다 커졌다면 Min로
        (Variables|Default|SetArray%20Index 0)
        (else
          (Variables|Default|SetArray%20Index (+ (Variables|Default|GetArray%20Index) 1))))
      (bind _output_get (Variables|Default|SetST%20Build (Utilities|Array|Get(acopy) (Variables|Default|GetST_BuildArray) (Variables|Default|GetArray%20Index))))
      (Components|StaticMesh|SetStaticMesh (Variables|Default|GetBuliding%20Preview) (.StaticMesh (Utilities|Struct|BreakST_Build _output_get)))
      (Default|UpdateInfo (Variables|Default|GetBuild%20Widget) (Variables|Default|GetST%20Build)))))

(event Input|MouseEvents|LeftMouseButton
  (params (Key :type Key%20Structure :default "None")))

(fn ConstructionScript)

(fn InitPawn
  (bind _assn_vrpawn (Utilities|Casting|CastToSN_VRPawn (Game|Player|GetPlayerPawn 0)))
  (bind _output_get (Variables|Default|SetOwn%20VRPawn _assn_vrpawn))
  (Variables|Default|SetWidgetInteractionRefLeft (Variables|/Game/Subnotica/GameMode/SN_VRPawn.SN_VRPawn_C|GetWidgetInteractionLeft _output_get))
  (Variables|Default|SetWidgetInteractionRefRight (Variables|/Game/Subnotica/GameMode/SN_VRPawn.SN_VRPawn_C|GetWidgetInteractionRight _output_get)))

(fn SetBuildingPreview
  (params (Preview%20Mesh :type Static%20Mesh%20Object%20Reference) (Preview%20Material :type Material%20Interface%20Object%20Reference))
  (bind _buliding_preview (Variables|Default|GetBuliding%20Preview))
  (bind _collision_box (Variables|Default|GetCollision%20Box))
  (bind _buliding_preview_2 (Variables|Default|GetBuliding%20Preview))
  (bind _staticmesh (Variables|/Script/Engine.StaticMeshComponent|GetStaticMesh _buliding_preview))
  (bind _returnvalue (StaticMesh|GetBounds _staticmesh))
  (Components|StaticMesh|SetStaticMesh (Variables|Default|GetBuliding%20Preview) Preview%20Mesh)
  (for _index (range 0 (- (Rendering|Material|GetNumMaterials _buliding_preview_2) 1))
    (Rendering|Material|SetMaterial _buliding_preview_2 _index Preview%20Material) ; Preview Material 로 변경
    (Components|Box|SetBoxExtent _collision_box (.boxextent _returnvalue) true) ; Collision Box 크기 Building Mesh 크기에 맞춤
    (Transformation|SetRelativeLocation _collision_box (Math|Vector|MakeVector 0.0 0.0 (.Z (Math|Vector|BreakVector (.origin _returnvalue)))) false false) ; 콜리전 높이 맞춰줌
  ))

(fn SetLocationBuildingPreview
  (bind _returnvalue (Transformation|GetActorLocation))
  (bind (_outhit _returnvalue_2) (Collision|LineTraceByChannel _returnvalue (+ _returnvalue (* (Transformation|GetActorForwardVector) 1e+03)) "TraceTypeQuery4" false 0 "ForDuration"))
  (if _returnvalue_2 ; 히트 되면 히트 위치에\n히트 안되면 트레이스 끝에 배치
    (if (Utilities|String|Contains (Utilities|GetDisplayName (.HitComponent (Collision|BreakHitResult _outhit))) "BuildCollision") ; Build Collision에 히트됐는가?
      (Variables|Default|SetImpact%20Point (.ImpactPoint (Collision|BreakHitResult _outhit)))
      (bind _collision (Class|BPIBuild|GetCollisionArray(Message) (.HitActor (Collision|BreakHitResult _outhit))))
      (bind _array_element (Utilities|Array|ForEachLoopwithBreak _collision :!label _label)
        (:LoopBody
          (if (== _array_element (.HitComponent (Collision|BreakHitResult _outhit)))
            (LocalVariables|SetCalculate%20Vector (- (Transformation|GetWorldLocation (.HitComponent (Collision|BreakHitResult _outhit))) (Transformation|GetActorLocation (.HitActor (Collision|BreakHitResult _outhit)))))
            (if (!= (.x (LocalVariables|GetCalculate%20Vector)) 0.0) ; X방향 콜리전인가?\nY방향 콜리전인가?\n(World)
              (bind _output_get (Variables|Default|SetBuild%20Location (CallFunction|GetBuildXPosition (.HitComponent (Collision|BreakHitResult _outhit)) (> (.x (LocalVariables|GetCalculate%20Vector)) 0.0))))
              (Transformation|SetWorldLocation (Variables|Default|GetBuliding%20Preview) _output_get false false)
              (goto _label Break)
              (else
                (bind _output_get_2 (Variables|Default|SetBuild%20Location (CallFunction|GetBuildYPosition (.HitComponent (Collision|BreakHitResult _outhit)) (> (.y (LocalVariables|GetCalculate%20Vector)) 0.0))))
                (Transformation|SetWorldLocation (Variables|Default|GetBuliding%20Preview) _output_get_2 false false)
                (goto _label Break)))))
        (:Completed
          (return true)))
      (else
        (bind _output_get_3 (Variables|Default|SetBuild%20Location (.ImpactPoint (Collision|BreakHitResult _outhit))))
        (Transformation|SetWorldLocation (Variables|Default|GetBuliding%20Preview) _output_get_3 false false)
        (return false)))
    (else
      (Transformation|SetWorldLocation (Variables|Default|GetBuliding%20Preview) (.TraceEnd (Collision|BreakHitResult _outhit)) false false)
      (return false))))

(fn CheckPossibleBuild
  (params (On%20Build%20Collision? :type Boolean))
  (if On%20Build%20Collision?
    ;[0.1146 0.1146 0.1146] Is Overlap Only BuildCollision?
    (bind _array_element (Utilities|Array|ForEachLoopwithBreak (Class|PrimitiveComponent|GetOverlappingComponents (Variables|Default|GetCollision%20Box)) :!label _label)
      (:LoopBody
        (if (Utilities|String|Contains (Utilities|GetDisplayName _array_element) "BuildCollision") ; BuildCollision 임?
          (LocalVariables|SetOnly%20BuildCollision? true)
          (else
            (LocalVariables|SetOnly%20BuildCollision? false)
            (goto _label Break))))
      (:Completed
        (return (LocalVariables|GetOnly%20BuildCollision?))))
    (else
      ;[0.1146 0.1146 0.1146] Is Valid Overlap?
      (if (not (or (Utilities|Array|IsValidIndex (Collision|GetOverlappingActors (Variables|Default|GetCollision%20Box) "/Script/Landscape.Landscape" :!class /Script/Engine.PrimitiveComponent)) (Utilities|Array|IsValidIndex (Collision|GetOverlappingActors (Variables|Default|GetCollision%20Box) "/Script/Engine.Actor" :!class /Script/Engine.PrimitiveComponent))))
        (return true)
        (else
          (return false))))))

(fn IsAxisGreaterThanDeadzone
  (params (AxisValue :type Float%20%28single-precision%29))
  (return (>= (Math|Float|Absolute(Float) AxisValue) (Variables|Default|GetAxisDeadzoneThreshold))))

(fn InitBuildArray
  (bind _outrownames (DataTable|GetDataTableRowNames "/Game/Subnotica/Data/DT_Build.DT_Build"))
  (for _array_element _outrownames
    (bind _returnvalue (Utilities|GetDataTableRow "/Game/Subnotica/Data/DT_Build.DT_Build" _array_element)
      (:then
        (Utilities|Array|Add (Variables|Default|GetST_BuildArray) _returnvalue)))))

(fn GetBuildYPosition
  (params (Target :type Scene%20Component%20Object%20Reference) (Forward? :type Boolean))
  (bind _returnvalue (Transformation|GetWorldLocation Target))
  (bind _returnvalue_2 (Transformation|GetWorldLocation Target))
  (if Forward?
    (return (Math|Vector|MakeVector (.x _returnvalue_2) (+ (.y _returnvalue_2) (/ (.Y (Math|Vector|BreakVector (.boxextent (StaticMesh|GetBounds (.StaticMesh (Utilities|Struct|BreakST_Build (Variables|Default|GetST%20Build))))))) 2.0)) (.z _returnvalue_2)))
    (else
      (return (Math|Vector|MakeVector (.x _returnvalue) (- (.y _returnvalue) (/ (.Y (Math|Vector|BreakVector (.boxextent (StaticMesh|GetBounds (.StaticMesh (Utilities|Struct|BreakST_Build (Variables|Default|GetST%20Build))))))) 2.0)) (.z _returnvalue))))))

(fn GetBuildXPosition
  (params (Target :type Scene%20Component%20Object%20Reference) (Forward? :type Boolean))
  (bind _returnvalue (Transformation|GetWorldLocation Target))
  (bind _returnvalue_2 (Transformation|GetWorldLocation Target))
  (if Forward?
    (return (Math|Vector|MakeVector (+ (.x _returnvalue_2) (/ (.Y (Math|Vector|BreakVector (.boxextent (StaticMesh|GetBounds (.StaticMesh (Utilities|Struct|BreakST_Build (Variables|Default|GetST%20Build))))))) 2.0)) (.y _returnvalue_2) (.z _returnvalue_2)))
    (else
      (return (Math|Vector|MakeVector (- (.x _returnvalue) (/ (.Y (Math|Vector|BreakVector (.boxextent (StaticMesh|GetBounds (.StaticMesh (Utilities|Struct|BreakST_Build (Variables|Default|GetST%20Build))))))) 2.0)) (.y _returnvalue) (.z _returnvalue))))))

(fn InitVariable
  (Utilities|FlowControl|Sequence
    (:then_0
      (bind _returnvalue (Utilities|GetDataTableRow "/Game/Subnotica/Data/DT_Build.DT_Build" "Build_01")
        (:then
          (bind _output_get (Variables|Default|SetST%20Build _returnvalue))
          (CallFunction|SetBuildingPreview (.StaticMesh (Utilities|Struct|BreakST_Build _output_get)) "/Game/Subnotica/Effect/Build/WM_GlassClean_a.WM_GlassClean_a"))))
    (:then_1
      (bind _returnvalue_2 (Utilities|GetDataTableRow "/Game/Subnotica/Data/DT_Item.DT_Item" "Scanner")
        (:then
          (bind _output_get_2 (Variables|Default|SetST_Item _returnvalue_2))
          (Development|PrintString (Utilities|String|ToString(Integer) (.ItemIndex (Utilities|Struct|BreakST_Item _output_get_2))) false false))))))

(fn CheckUnderWater
  (bind _ocean (Variables|Default|GetOcean))
  (Utilities|IsValid _ocean
    (:Is%20Valid
      (if (> (- (.z (Transformation|GetActorLocation _ocean)) (.z (Transformation|GetWorldLocation (Variables|Default|GetBuliding%20Preview)))) 0.0)
        (return true)
        (else
          (return false))))))

(fn DragEvent
  (return false))

(fn DropItem
  (Variables|Default|SetInventory%20Widget 0)
  (Variables|Default|SetWatch 0)
  (return false))

(fn GetItem
  (params (Own%20Pawn :type SN%20VR%20Pawn%20Object%20Reference) (Inventory%20Widget :type Inventory%20Widget%20Object%20Reference) (Watch :type Watch%20Object%20Reference))
  (Variables|Default|SetInventory%20Widget Inventory%20Widget)
  (bind _output_get (Variables|Default|SetWatch Watch))
  (Variables|/Game/Subnotica/BluePrint/Watch/Watch.Watch_C|SetScanner _output_get self)
  (return false))

(fn PressTrigger
  (return false))

(fn RealeseTrigger
  (return false))