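; Grabbable VR fish pawn that wanders underwater and becomes an inventory item when dropped with a valid inventory widget.
; Within range of the player and while not held, it eases rotation toward its velocity and swims toward random box points below the ocean surface.
; Hitting anything other than another fish picks a new heading.
; Rising above the water or straying from its Spawner teleports it to a random point in the spawner box.
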(event OnComponentHit(CollisionComponent)
  (params (HitComponent :type Primitive%20Component%20Object%20Reference) (OtherActor :type Actor%20Object%20Reference) (OtherComp :type Primitive%20Component%20Object%20Reference) (NormalImpulse :type Vector :default "0, 0, 0") (Hit :type Hit%20Result%20Structure%20%28by%20ref%29))
  ;[0.125 0.125 0.125] Hit Event
  (Utilities|Casting|CastToBP_FishFlock OtherActor
    (:CastFailed
      (CallFunction|-FindNewLocationandDirection))))

(event OnDropped(GrabComponent)
  (bind _inventory_widget (Variables|Default|GetInventory%20Widget))
  (Variables|Default|SetIs%20Grab false)
  (Utilities|IsValid _inventory_widget
    (:Is%20Valid
      (Default|UpdateItem _inventory_widget (Variables|Default|GetST%20Item))
      (Actor|DestroyActor))))

(event OnGrabbed(GrabComponent)
  (params (Motion%20Controller :type Motion%20Controller%20Component%20Object%20Reference))
  (Variables|Default|SetIs%20Grab true))

(event EventTick
  (params (DeltaSeconds :type Float%20%28single-precision%29))
  (bind _spawner (Variables|Default|GetSpawner))
  (bind _box (Variables|/Game/Subnotica/BluePrint/Spawn_ItemFish.Spawn_ItemFish_C|GetBox _spawner))
  ;[0.125 0.125 0.125] Tick
  (if (< (Transformation|GetDistanceTo (Game|Player|GetPlayerPawn 0)) 4e+03)
    (if (not (Variables|Default|GetIs%20Grab))
      (Variables|Default|SetCur%20Delta%20Seconds DeltaSeconds)
      (CallFunction|-LookingForward)
      (Utilities|FlowControl|Sequence
        (:then_0
          (Utilities|FlowControl|DoOnce false
            (:Completed
              (CallFunction|-FindNewLocationandDirection))))
        (:then_1
          _))
      (Pawn|Input|AddMovementInput (Variables|Default|GetAverage_Acceleration) (Variables|Default|GetSpeed_Scale) false)
      (if (== (Math|Float|Truncate (Variables|Default|GetCur%20Delta%20Seconds)) (Math|Float|Truncate (Math|Random|RandomFloatinRange 3.0 1e+01)))
        (CallFunction|-FindNewLocationandDirection)
        (Variables|Default|SetSpeed_Scale (Math|Random|RandomFloatinRange 0.5 1.0))
        (else
          (Variables|Default|SetSpeed_Scale (Math|Random|RandomFloatinRange 0.7 1.0))))
      (Utilities|FlowControl|Sequence
        (:then_0
          (if (>= (- (.z (Transformation|GetActorLocation)) (.z (Transformation|GetActorLocation (Variables|Default|GetOcean)))) 0.0)
            (Transformation|SetActorLocation (Math|Random|RandomPointinBoundingBox (Transformation|GetWorldLocation _box) (Components|Box|GetScaledBoxExtent _box)) false false :!label _label)))
        (:then_1
          (if (> (Transformation|GetDistanceTo (Variables|Default|GetSpawner)) 2e+03)
            (goto _label)))))))

(event EventBeginPlay
  ;[0.125 0.125 0.125] Begin
  (Components|StaticMesh|SetStaticMesh (Variables|GetMeshComponent) (.ItemMesh (Utilities|Struct|BreakST_Item (Variables|Default|GetST%20Item))))
  (bind _assn_game_mode (Utilities|Casting|CastToSN_GameMode (Game|GetGameMode)))
  (Default|FishControllerPossess _assn_game_mode self)
  (bind _returnvalue (Actor|GetActorOfClass "/Game/CartoonWaterShader/Blueprints/CartoonWaterBlueprints/BP_CartoonWater_Ocean.BP_CartoonWater_Ocean_C"))
  (Utilities|IsValid _returnvalue
    (:Is%20Valid
      (Variables|Default|SetOcean _returnvalue)
      (bind _assn_vrpawn (Utilities|Casting|CastToSN_VRPawn (Game|Player|GetPlayerPawn 0)))
      (Variables|Default|SetOwn%20VRPawn _assn_vrpawn))))

(event EventDestroyed)

(fn ConstructionScript)

(fn -LookingForward
  (Transformation|SetActorRotation (Math|Interpolation|Ease "EaseInOut" 0.1 (Transformation|GetActorRotation) (Math|Rotator|MakeRotfromX (Math|Vector|Normalize (Transformation|GetVelocity))) true))
  (return))

(fn -FindNewLocationandDirection
  (bind _box (Variables|Default|GetBox))
  (bind _returnvalue (Transformation|GetWorldLocation _box))
  (bind _boxextent (Variables|/Script/Engine.BoxComponent|GetBoxExtent _box))
  (bind _returnvalue_2 (Math|Random|RandomPointinBoundingBox _returnvalue _boxextent))
  (if (> (.Z (Math|Vector|BreakVector _returnvalue_2)) (.z (Transformation|GetActorLocation (Variables|Default|GetOcean))))
    (Utilities|Time|SetTimerbyFunctionName 0 "- Find New Location and Direction" 0.01)
    (else
      (Variables|Default|SetTarget_Location _returnvalue_2)
      (Variables|Default|SetAverage_Acceleration (Math|Vector|Normalize (- _returnvalue_2 (Transformation|GetActorLocation))))
      (return))))

(fn DragEvent
  (return false))

(fn DropItem
  (Variables|Default|SetInventory%20Widget 0))

(fn GetItem
  (params (Own%20Pawn :type SN%20VR%20Pawn%20Object%20Reference) (Inventory%20Widget :type Inventory%20Widget%20Object%20Reference) (Watch :type Watch%20Object%20Reference))
  (Variables|Default|SetInventory%20Widget Inventory%20Widget))

(fn PressTrigger
  (return false))

(fn RealeseTrigger
  (return false))