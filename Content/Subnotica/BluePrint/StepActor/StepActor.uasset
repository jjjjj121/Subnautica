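; StepActor is an actor representing one step in the game's step-based progression, tied to SN_GameState.
; On BeginPlay it caches the VR pawn and game state, then binds to the game state's step-change dispatcher.
; When the broadcast step matches MyStep, it prints a debug message and runs BeginStep, which plays optional 2D background sound.
; EndStep advances the game state to NextStep, and construction sets a text label.
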(event EventBeginPlay
  (bind _assn_vrpawn (Utilities|Casting|CastToSN_VRPawn (Game|Player|GetPlayerPawn 0)))
  (Variables|Default|SetSN%20VRPawn _assn_vrpawn)
  (bind _assn_game_state (Utilities|Casting|CastToSN_GameState (Game|GetGameState)))
  (Variables|Default|SetGame%20State _assn_game_state)
  (EventDispatchers|BindEventtoEventDispatcherChangeStep _assn_game_state (EventDispatchers|CreateEvent :!event EventChangeStep)))

(fn ConstructionScript
  (Rendering|Components|TextRender|SetText (Variables|Default|GetTextRender) (Variables|Default|GetText)))

(fn BeginStep
  (bind _background_sound (Variables|Default|GetBackGround%20Sound)
    (:then
      (Audio|PlaySound2D _background_sound 1.0 1.0 0.0 0 0))
    (:else)))

(fn EndStep
  (Default|SetStep (Variables|Default|GetGame%20State) (Variables|Default|GetNext%20Step)))

(fn EventChangeStep
  (params (Step :type Byte :default 0))
  (if (== Step (Variables|Default|GetMy%20Step))
    (Development|PrintString (Utilities|String|Append (Utilities|GetDisplayName self) " -  " "My Step   :  " (Utilities|String|ToString(Byte) (Variables|Default|GetMy%20Step)) "    /    Cur Step :  " (Utilities|String|ToString(Byte) Step)) true true "(R=0.087081,G=0.000000,B=1.000000,A=1.000000)" 3e+01)
    (CallFunction|BeginStep)))