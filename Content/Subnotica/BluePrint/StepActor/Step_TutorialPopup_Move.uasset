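; Tutorial step actor for the move popup, which completes once the player moves.
; Loop Func stores the SNVR pawn's location and starts a fast looping timer that polls Check Next Time by function name.
; Check Next Time compares the stored location with player pawn 0's location and calls End Step when they differ beyond a small tolerance.
; Both overrides skip their parent implementations.
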(event EventBeginPlay
  (|CallParentFunction) ; 지금 이 노드는 비활성 상태입니다. \n핀을 끌어서 다른 노드를 연결하면 활성화됩니다.
)

(event Collision|EventActorBeginOverlap
  (params (OtherActor :type Actor%20Object%20Reference))
  (|CallParentFunction OtherActor) ; 지금 이 노드는 비활성 상태입니다. \n핀을 끌어서 다른 노드를 연결하면 활성화됩니다.
)

(event EventTick
  (params (DeltaSeconds :type Float%20%28single-precision%29))
  (|CallParentFunction DeltaSeconds) ; 지금 이 노드는 비활성 상태입니다. \n핀을 끌어서 다른 노드를 연결하면 활성화됩니다.
)

(fn ConstructionScript
  (|CallParentFunction))

(fn CheckNextTime
  (if (Math|Vector|NotEqual(Vector) (Variables|Default|GetPlayer%20Location) (Transformation|GetActorLocation (Game|Player|GetPlayerPawn 0)) 0.01) ; 이동 시 엔드
    (CallFunction|EndStep)))

(fn LoopFunc
  (Variables|Default|SetPlayer%20Location (Transformation|GetActorLocation (Variables|Default|GetSN%20VRPawn)))
  (Utilities|Time|SetTimerbyFunctionName 0 "Check Next Time" 0.01 true))