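; Tutorial step actor that shows a text popup with optional audio and waits for the VR player to complete the current watch, scanner or SeaGlide task.
; BeginPlay fills and hides the widget; BeginStep reveals it, plays the sound and binds an audio-finished event.
; LoopFunc starts a fast looping timer that polls the pawn's watch and tool state per step type.
; A met condition calls EndStep, which destroys the actor.
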(event EventBeginPlay
  (|CallParentFunction)
  (Rendering|SetVisibility (Variables|Default|GetWidget) false false)
  (bind _astutorial_start (Utilities|Casting|CastToTutorial_Start (UserInterface|GetWidget (Variables|Default|GetWidget))))
  (bind _output_get (Variables|Default|SetTutorial%20Widget _astutorial_start))
  (Default|SetText _output_get (Variables|Default|GetInfo%20Text)))

(event Collision|EventActorBeginOverlap
  (params (OtherActor :type Actor%20Object%20Reference)))

(event EventTick
  (params (DeltaSeconds :type Float%20%28single-precision%29)))

(fn ConstructionScript
  (|CallParentFunction)
  (Audio|Components|Audio|SetSound (Variables|Default|GetAudio) (Variables|Default|GetNew%20Sound)))

(fn BeginStep
  (bind _audio (Variables|Default|GetAudio))
  (|CallParentFunction)
  (Rendering|SetVisibility (Variables|Default|GetWidget) true false)
  (Utilities|IsValid (Variables|/Script/Engine.AudioComponent|GetSound _audio)
    (:Is%20Valid
      (Audio|Components|Audio|Play _audio 0.0)
      (EventDispatchers|BindEventtoOnAudioFinished _audio (EventDispatchers|CreateEvent :!event LoopFunc)))))

(fn LoopFunc
  (Utilities|Time|SetTimerbyFunctionName 0 "Check Next Time" 0.01 true))

(fn CheckNextTime
  (bind _sn_vrpawn (Variables|Default|GetSN%20VRPawn))
  (bind _watch (Variables|/Game/Subnotica/GameMode/SN_VRPawn.SN_VRPawn_C|GetWatch _sn_vrpawn))
  (Development|PrintString "Cehck" false false)
  (switch Utilities|FlowControl|Switch|SwitchonEnum_GameStep (Variables|Default|GetMy%20Step)
    (:NewEnumerator2
      (Utilities|IsValid (Variables|/Game/Subnotica/GameMode/SN_VRPawn.SN_VRPawn_C|GetWatch (Variables|Default|GetSN%20VRPawn)) ; 어태치 했을 때
        (:Is%20Valid
          (CallFunction|EndStep :!label _label))))
    (:NewEnumerator5
      (if (Rendering|IsVisible (Variables|/Game/Subnotica/BluePrint/Watch/Watch.Watch_C|GetWidget_Menu (Variables|/Game/Subnotica/GameMode/SN_VRPawn.SN_VRPawn_C|GetWatch (Variables|Default|GetSN%20VRPawn)))) ; 메뉴 열었을 때
        (goto _label)))
    (:NewEnumerator6
      (if (and (Variables|/Game/Subnotica/BluePrint/Watch/Watch.Watch_C|GetIs%20Get%20SeaGlide _watch) (Variables|/Game/Subnotica/BluePrint/Watch/Watch.Watch_C|GetIs%20Get%20Scanner _watch)) ; 둘 다 귀속되었을 때
        (goto _label)))
    (:NewEnumerator3
      (Variables|/Game/Subnotica/BluePrint/Watch/Watch.Watch_C|GetScanner (Variables|/Game/Subnotica/GameMode/SN_VRPawn.SN_VRPawn_C|GetWatch (Variables|Default|GetSN%20VRPawn))
        (:then
          (goto _label))
        (:else)))
    (:NewEnumerator4
      (Variables|/Game/Subnotica/BluePrint/Watch/Watch.Watch_C|GetSeaGlide (Variables|/Game/Subnotica/GameMode/SN_VRPawn.SN_VRPawn_C|GetWatch (Variables|Default|GetSN%20VRPawn))
        (:then
          (goto _label))
        (:else)))
    (:NewEnumerator10
      (bind _scanner (Variables|/Game/Subnotica/BluePrint/Watch/Watch.Watch_C|GetScanner (Variables|/Game/Subnotica/GameMode/SN_VRPawn.SN_VRPawn_C|GetWatch (Variables|Default|GetSN%20VRPawn)))
        (:then
          (Development|PrintString "@@@@@" false false)
          (if (Variables|/Game/Subnotica/BluePrint/Building_Scanner.Building_Scanner_C|GetIs%20Building%20Mode _scanner)
            (goto _label)))
        (:else
          (Development|PrintString "$$$$#$#$" false false "(R=1.000000,G=0.036710,B=0.000000,A=1.000000)"))))
    (:NewEnumerator11
      (if (Rendering|IsVisible (Variables|/Game/Subnotica/BluePrint/Watch/Watch.Watch_C|GetScan (Variables|/Game/Subnotica/GameMode/SN_VRPawn.SN_VRPawn_C|GetWatch (Variables|Default|GetSN%20VRPawn))))
        (goto _label)))
    (:NewEnumerator12
      (bind _seaglide (Variables|/Game/Subnotica/BluePrint/Watch/Watch.Watch_C|GetSeaGlide (Variables|/Game/Subnotica/GameMode/SN_VRPawn.SN_VRPawn_C|GetWatch (Variables|Default|GetSN%20VRPawn)))
        (:then
          (if (Variables|/Game/Subnotica/BluePrint/SeaGlide.SeaGlide_C|GetIs%20Grab%20All%20Handle? _seaglide)
            (goto _label)))
        (:else)))))

(fn EndStep
  (|CallParentFunction)
  (Actor|DestroyActor))