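; Spawner actor that keeps a population of BP_FishFlock actors inside its box volume in a VR game.
; On BeginPlay it caches the SN_VRPawn player and DT_Item rows named with "Fish", then spawns twenty flocks after one short delay.
; Each spawn gets a random point, a random fish row, the player and the spawner.
; A destroy binding on each flock appears to trigger a replacement spawn through DestroyFish.
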(event EventBeginPlay
  (CallFunction|InitPawn)
  (CallFunction|InitFish)
  (Utilities|ForLoopDelay 1 20 0.3
    (:Loop%20Body
      (CallFunction|RandomSpawn))))

(fn ConstructionScript)

(fn RandomSpawn
  (bind _box (Variables|Default|GetBox))
  (bind _returnvalue (Utilities|GetDataTableRow "/Game/Subnotica/Data/DT_Item.DT_Item" (CallFunction|GetRandomRowName))
    (:then
      (bind _returnvalue_2 (Game|SpawnActorfromClass "/Game/Subnotica/BluePrint/BP_FishFlock.BP_FishFlock_C" (Math|Transform|MakeTransform (Math|Random|RandomPointinBoundingBox (Transformation|GetWorldLocation _box) (Components|Box|GetScaledBoxExtent _box)) "0, 0, 0" "1,1,1") "AdjustIfPossibleButAlwaysSpawn" 0 _returnvalue (Variables|Default|GetPlayer) self 0))
      (Game|BindEventtoOnDestroyed _returnvalue_2 (EventDispatchers|CreateEvent :!event DestroyFish)))))

(fn DestroyFish
  (params (DestroyedActor :type Actor%20Object%20Reference))
  (CallFunction|RandomSpawn))

(fn InitFish
  (bind _outrownames (DataTable|GetDataTableRowNames "/Game/Subnotica/Data/DT_Item.DT_Item"))
  (for _array_element _outrownames
    (if (Utilities|String|Contains (Utilities|String|ToString(Name) _array_element) "Fish")
      (Utilities|Array|Add (Variables|Default|GetFish%20Row%20Names) _array_element))))

(fn GetRandomRowName
  (return (.OutItem (Utilities|Array|Random (Variables|Default|GetFish%20Row%20Names)))))

(fn InitPawn
  (bind _assn_vrpawn (Utilities|Casting|CastToSN_VRPawn (Game|Player|GetPlayerPawn 0)))
  (Variables|Default|SetPlayer _assn_vrpawn))