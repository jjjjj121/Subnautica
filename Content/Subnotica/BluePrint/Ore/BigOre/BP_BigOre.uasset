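; BP_BigOre is a large ore deposit that dissolves while a Watch actor overlaps its mesh, then breaks into a random small ore.
; Overlap begin starts a looping timer that lowers the "Desolve" scalar on a dynamic material until a threshold, where it spawns the small ore above itself and destroys itself.
; Ending the overlap early stops the timer and resets the dissolve.
; Drag, drop and get-item functions are stubs returning false.
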(event OnComponentBeginOverlap(StaticMesh)
  (params (OverlappedComponent :type Primitive%20Component%20Object%20Reference) (OtherActor :type Actor%20Object%20Reference) (OtherComp :type Primitive%20Component%20Object%20Reference) (OtherBodyIndex :type Integer) (bFromSweep :type Boolean) (SweepResult :type Hit%20Result%20Structure%20%28by%20ref%29))
  (Development|PrintString (Utilities|String|Append (Utilities|GetDisplayName OtherActor) (Utilities|GetDisplayName OtherComp)) true true "(R=1.000000,G=0.000000,B=0.865883,A=1.000000)" 5.0)
  (Utilities|Casting|CastToWatch OtherActor)
  (CallFunction|PressTrigger))

(event OnComponentEndOverlap(StaticMesh)
  (params (OverlappedComponent :type Primitive%20Component%20Object%20Reference) (OtherActor :type Actor%20Object%20Reference) (OtherComp :type Primitive%20Component%20Object%20Reference) (OtherBodyIndex :type Integer))
  (Utilities|Casting|CastToWatch OtherActor)
  (CallFunction|RealeseTrigger))

(event EventBeginPlay
  (bind _returnvalue (Rendering|Material|CreateDynamicMaterialInstance (Variables|Default|GetStaticMesh) 0 (Rendering|Material|GetMaterial (Variables|Default|GetStaticMesh) 0) "None" :!class /Script/Engine.PrimitiveComponent))
  (Variables|Default|SetMaterial%20Instance _returnvalue))

(fn ConstructionScript)

(fn DesolveActor
  (if (<= (Variables|Default|GetValue) -1.0)
    (Utilities|Time|ClearTimerbyFunctionName 0 "Desolve Actor")
    (Game|SpawnActorfromClass (.OutItem (Utilities|Array|Random (Variables|Default|GetSmall%20Ore%20Class))) (Math|Transform|MakeTransform (+ (Transformation|GetActorLocation) (* (Transformation|GetActorUpVector) 5e+01)) "0, 0, 0" "1,1,1") "Undefined" 0 0)
    (Actor|DestroyActor)
    (else
      (bind _output_get (Variables|Default|SetValue (- (Variables|Default|GetValue) 0.02)))
      (Rendering|Material|SetScalarParameterValue (Variables|Default|GetMaterial%20Instance) "Desolve" _output_get :!class /Script/Engine.MaterialInstanceDynamic))))

(fn DragEvent
  (return false))

(fn DropItem
  (return false))

(fn GetItem
  (params (Own%20Pawn :type SN%20VR%20Pawn%20Object%20Reference) (Inventory%20Widget :type Inventory%20Widget%20Object%20Reference) (Watch :type Watch%20Object%20Reference))
  (return false))

(fn PressTrigger
  (Utilities|Time|SetTimerbyFunctionName 0 "Desolve Actor" 0.05 true))

(fn RealeseTrigger
  (Utilities|Time|ClearTimerbyFunctionName 0 "Desolve Actor")
  (bind _output_get (Variables|Default|SetValue 0.7))
  (Rendering|Material|SetScalarParameterValue (Variables|Default|GetMaterial%20Instance) "Desolve" _output_get :!class /Script/Engine.MaterialInstanceDynamic))