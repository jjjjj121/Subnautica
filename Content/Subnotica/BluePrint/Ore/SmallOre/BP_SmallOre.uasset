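; BP_SmallOre is a grabbable VR small ore pickup that can be stored in the player's inventory.
; On BeginPlay it scans DT_Item for row names containing OreName and caches the matching row as its item data.
; GetItem stores an inventory widget reference and DropItem clears it; releasing the GrabComponent while that reference is valid adds the item and destroys the actor.
; Drag and trigger functions are stubs, and grab haptics are disconnected.
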(event OnDropped(GrabComponent)
  (bind _inventory_widget (Variables|Default|GetInventory%20Widget))
  (Utilities|IsValid _inventory_widget
    (:Is%20Valid
      (Default|UpdateItem _inventory_widget (Variables|Default|GetST_Item))
      (Actor|DestroyActor))))

(event OnGrabbed(GrabComponent)
  (params (Motion%20Controller :type Motion%20Controller%20Component%20Object%20Reference)))

(event EventBeginPlay
  (bind _outrownames (DataTable|GetDataTableRowNames "/Game/Subnotica/Data/DT_Item.DT_Item"))
  (for _array_element _outrownames
    (if (Utilities|String|Contains (Utilities|String|ToString(Name) _array_element) (Variables|Default|GetOre%20Name))
      (bind _returnvalue (Utilities|GetDataTableRow "/Game/Subnotica/Data/DT_Item.DT_Item" _array_element)
        (:then
          (Variables|Default|SetST_Item _returnvalue))))))

(event Collision|EventActorBeginOverlap
  (params (OtherActor :type Actor%20Object%20Reference)))

(event EventTick
  (params (DeltaSeconds :type Float%20%28single-precision%29)))

(fn ConstructionScript)

(fn DragEvent
  (return false))

(fn DropItem
  (Variables|Default|SetInventory%20Widget 0))

(fn GetItem
  (params (Own%20Pawn :type SN%20VR%20Pawn%20Object%20Reference) (Inventory%20Widget :type Inventory%20Widget%20Object%20Reference) (Watch :type Watch%20Object%20Reference))
  (Variables|Default|SetInventory%20Widget Inventory%20Widget))

(fn PressTrigger
  (return false))

(fn RealeseTrigger
  (return false))