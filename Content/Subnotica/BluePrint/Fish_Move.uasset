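; Fish spawner actor that gives five Niagara fish components distinct random effects from FishGroup and periodically relocates them.
; BeginPlay sets short per-fish timers, then StartMove immediately replaces them with looping timers at random 15–25 second intervals.
; Each timer jumps its fish to a random navigable point within its own radius around the actor.
; Move Fish_03 and 04 also target Fish2, so Fish3 and Fish4 never move.
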(event EventBeginPlay
  (bind _fish_group (Variables|Default|GetFish_Group))
  (for _index (range 1 5)
    (bind _output_get (Variables|Default|SetPrev%20Fish (.OutItem (Utilities|Array|Random _fish_group))))
    (Utilities|Array|RemoveItem _fish_group _output_get)
    (switch int _index
      (:1
        (Class|NiagaraComponent|SetAsset (Variables|Default|GetFish_0) _output_get true))
      (:2
        (Class|NiagaraComponent|SetAsset (Variables|Default|GetFish_1) _output_get true))
      (:3
        (Class|NiagaraComponent|SetAsset (Variables|Default|GetFish_2) _output_get true))
      (:4
        (Class|NiagaraComponent|SetAsset (Variables|Default|GetFish_3) _output_get true))
      (:5
        (Class|NiagaraComponent|SetAsset (Variables|Default|GetFish_4) _output_get true))))
  (Utilities|Time|SetTimerbyFunctionName 0 "Move Fish_00" 0.1)
  (Utilities|Time|SetTimerbyFunctionName 0 "Move Fish_01" 0.01)
  (Utilities|Time|SetTimerbyFunctionName 0 "Move Fish_02" 1.0)
  (Utilities|Time|SetTimerbyFunctionName 0 "Move Fish_03" 2.0)
  (Utilities|Time|SetTimerbyFunctionName 0 "Move Fish_04" 0.5)
  (CallFunction|StartMove))

(event Collision|EventActorBeginOverlap
  (params (OtherActor :type Actor%20Object%20Reference)))

(event EventTick
  (params (DeltaSeconds :type Float%20%28single-precision%29)))

(fn ConstructionScript)

(fn MoveFish00
  (Transformation|SetWorldLocation (Variables|Default|GetFish_0) (.RandomLocation (Class|NavigationSystemV1|GetRandomPointinNavigableRadius (Transformation|GetActorLocation) 2e+03 0 0)) false false))

(fn MoveFish01
  (Transformation|SetWorldLocation (Variables|Default|GetFish_1) (.RandomLocation (Class|NavigationSystemV1|GetRandomPointinNavigableRadius (Transformation|GetActorLocation) 5e+02 0 0)) false false))

(fn MoveFish02
  (Transformation|SetWorldLocation (Variables|Default|GetFish_2) (.RandomLocation (Class|NavigationSystemV1|GetRandomPointinNavigableRadius (Transformation|GetActorLocation) 2e+03 0 0)) false false))

(fn StartMove
  (Utilities|Time|SetTimerbyFunctionName 0 "Move Fish_00" (Math|Conversions|ToFloat(Integer) (Math|Random|RandomIntegerinRange 15 25)) true)
  (Utilities|Time|SetTimerbyFunctionName 0 "Move Fish_01" (Math|Conversions|ToFloat(Integer) (Math|Random|RandomIntegerinRange 15 25)) true)
  (Utilities|Time|SetTimerbyFunctionName 0 "Move Fish_02" (Math|Conversions|ToFloat(Integer) (Math|Random|RandomIntegerinRange 15 25)) true)
  (Utilities|Time|SetTimerbyFunctionName 0 "Move Fish_03" (Math|Conversions|ToFloat(Integer) (Math|Random|RandomIntegerinRange 15 25)) true)
  (Utilities|Time|SetTimerbyFunctionName 0 "Move Fish_04" (Math|Conversions|ToFloat(Integer) (Math|Random|RandomIntegerinRange 15 25)) true))

(fn MoveFish03
  (Transformation|SetWorldLocation (Variables|Default|GetFish_2) (.RandomLocation (Class|NavigationSystemV1|GetRandomPointinNavigableRadius (Transformation|GetActorLocation) 1.5e+03 0 0)) false false))

(fn MoveFish04
  (Transformation|SetWorldLocation (Variables|Default|GetFish_2) (.RandomLocation (Class|NavigationSystemV1|GetRandomPointinNavigableRadius (Transformation|GetActorLocation) 1e+03 0 0)) false false))